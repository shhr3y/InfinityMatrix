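; BP_Enemy is an enemy actor that resolves collisions with the player and bullets through overlap events on its EnemyObject component.
; Touching BP_Player deducts player health, destroys the enemy and plays a camera shake at its location.
; Overlapping a BP_Bullet instead awards score to player pawn 0, spawns an offset Niagara explosion and destroys the enemy.
; It has no movement or tick logic of its own.
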(event `self.EnemyObject.OnComponentBeginOverlap`
  (params (OverlappedComponent :type "PrimitiveComponent Object Reference") (OtherActor :type "Actor Object Reference") (OtherComp :type "PrimitiveComponent Object Reference") (OtherBodyIndex :type Integer) (bFromSweep :type Boolean) (SweepResult :type "HitResult Structure (by ref)"))
  (bind (_x _y _z) (`KismetMathLibrary.BreakVector3f` (`SceneComponent.K2_GetComponentLocation` OverlappedComponent)))
  (bind _asbp_player (cast `/Game/InfiniteMatrix/Blueprints/BP_Player` OtherActor)
    (:`then`
      (bind _output_get (set `self.User Ref` _asbp_player))
      (`/Game/InfiniteMatrix/Blueprints/BP_Player.UpdateUserHealth` _output_get -2)
      (`self.K2_DestroyActor`)
      (`GameplayStatics.PlayWorldCameraShake` "/Game/InfiniteMatrix/Blueprints/BP_CameraShake.BP_CameraShake_C" (`self.K2_GetActorLocation`) 0.0 500.0))
    (:`CastFailed`
      (cast `/Game/InfiniteMatrix/Blueprints/BP_Bullet` OtherActor)
      (bind _asbp_player_2 (cast `/Game/InfiniteMatrix/Blueprints/BP_Player` (`GameplayStatics.GetPlayerPawn` 0)))
      (`/Game/InfiniteMatrix/Blueprints/BP_Player.UpdateUserScore` _asbp_player_2 5)
      (`NiagaraFunctionLibrary.SpawnSystemAtLocation` "/Game/InfiniteMatrix/VFX/NS_Explosion.NS_Explosion" (`KismetMathLibrary.MakeVector` _x (- _y 300.0) (+ _z 50.0)))
      (`self.K2_DestroyActor`))))

(fn `UserConstructionScript`)