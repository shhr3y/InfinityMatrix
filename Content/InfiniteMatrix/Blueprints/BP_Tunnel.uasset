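; BP_Tunnel is a tunnel segment with a rotating obstacle wall that the player passes through.
; RandomizeWall picks one of four hole meshes and a random roll, and Tick keeps the wall spinning at RotateSpeed.
; Touching the wall costs the player one health and plays a camera shake.
; Reaching TriggerZone adds a point, asks TunnelSpawner to spawn another tunnel, then destroys this one.
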(event `self.ReceiveTick`
  (params (DeltaSeconds :type "Float (single-precision)"))
  (`SceneComponent.K2_AddLocalRotation` (`self.WallMesh`) (`KismetMathLibrary.MakeRotator` (* DeltaSeconds (`self.RotateSpeed`))) false false))

(event `self.TriggerZone.OnComponentBeginOverlap`
  (params (OverlappedComponent :type "PrimitiveComponent Object Reference") (OtherActor :type "Actor Object Reference") (OtherComp :type "PrimitiveComponent Object Reference") (OtherBodyIndex :type Integer) (bFromSweep :type Boolean) (SweepResult :type "HitResult Structure (by ref)"))
  (bind _asbp_player (cast `/Game/InfiniteMatrix/Blueprints/BP_Player` OtherActor))
  (set `self.User Ref` _asbp_player)
  (`|ExecutionSequence`
    (:`then_0`
      (`/Game/InfiniteMatrix/Blueprints/BP_Player.UpdateUserScore` (`self.User Ref`) 1))
    (:`then_1`
      (`/Game/InfiniteMatrix/Blueprints/BP_TunnerSpawner.Spawn Tunnel at Spawn Point` (`self.TunnelSpawner`))
      (`self.K2_DestroyActor`))))

(event `self.WallMesh.OnComponentBeginOverlap`
  (params (OverlappedComponent :type "PrimitiveComponent Object Reference") (OtherActor :type "Actor Object Reference") (OtherComp :type "PrimitiveComponent Object Reference") (OtherBodyIndex :type Integer) (bFromSweep :type Boolean) (SweepResult :type "HitResult Structure (by ref)"))
  (bind _asbp_player (cast `/Game/InfiniteMatrix/Blueprints/BP_Player` OtherActor))
  (bind _output_get (set `self.User Ref` _asbp_player))
  (`/Game/InfiniteMatrix/Blueprints/BP_Player.UpdateUserHealth` _output_get -1)
  (`GameplayStatics.PlayWorldCameraShake` "/Game/InfiniteMatrix/Blueprints/BP_CameraShake.BP_CameraShake_C" (`self.K2_GetActorLocation` _output_get) 0.0 500.0))

(fn `RandomizeWall`
  (bind _wallmesh (`self.WallMesh`))
  (`StaticMeshComponent.SetStaticMesh` _wallmesh (select `int` (`KismetMathLibrary.RandomIntegerInRange` 0 3) :`0` "/Game/InfiniteMatrix/Meshes/SM_Hole_01.SM_Hole_01" :`1` "/Game/InfiniteMatrix/Meshes/SM_Hole_02.SM_Hole_02" :`2` "/Game/InfiniteMatrix/Meshes/SM_Hole_03.SM_Hole_03" :`3` "/Game/InfiniteMatrix/Meshes/SM_Hole_04.SM_Hole_04" :!type "StaticMesh Object Reference"))
  (`SceneComponent.K2_AddLocalRotation` _wallmesh (`KismetMathLibrary.MakeRotator` (`KismetMathLibrary.RandomFloatInRange` 0.0 360.0)) false false))

(fn `UserConstructionScript`)